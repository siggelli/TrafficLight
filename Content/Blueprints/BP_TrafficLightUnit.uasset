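; BP_TrafficLightUnit is a traffic light unit that shows one Red, Yellow or Green signal at a time across its three lamps.
; SetSignal loops over the three child actor lamps, each cast to BP_TraffictLight, and calls ChangeColor on them.
; The lamp matching the signal gets its color from the CollorSettings color map, while the others turn black.
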(event Custom|SetSignal
  (params (Signal :type E_LightColor%20Enum :default "NewEnumerator0"))
  (for (_array_element _array_index) (Utilities|Array|MakeArray (Variables|Default|GetRedLight) (Variables|Default|GetYellowLight) (Variables|Default|GetGreenLight))
    (bind _asbp_traffict_light (Utilities|Casting|CastToBP_TraffictLight (Variables|/Script/Engine.ChildActorComponent|GetChildActor _array_element)))
    (if (== _array_index (Utilities|Select :Index Signal :NewEnumerator0 0 :NewEnumerator1 1 :NewEnumerator2 2))
      (Default|ChangeColor _asbp_traffict_light (.Value (Utilities|Map|Find (.colormap (Variables|Default|GetCollorSettings)) Signal)))
      (else
        (Default|ChangeColor _asbp_traffict_light)))))

(fn ConstructionScript)